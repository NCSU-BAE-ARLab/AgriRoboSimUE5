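; CameraRobot Blueprint is a networked robot actor that connects to a game server on BeginPlay and moves its Cube component from incoming byte messages.
; Its message-processing override decodes 24-byte messages as six floats for world location and rotation.
; Three-byte messages map each byte directly to a location axis, leaving the rotation input at its default.
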(event `self.ReceiveBeginPlay`
  (`self.ConnectToGameServer`))

(event `self.ReceiveTick`
  (params (DeltaSeconds :type "Float (single-precision)")))

(fn `MessageProcessImplementableEvent`
  (returns (ReturnValue :type Boolean))
  (bind _messagebytes (`self.MessageBytes`))
  (bind _returnvalue (`KismetArrayLibrary.Array_Length` _messagebytes))
  (`/Engine/EditorBlueprintResources/StandardMacros.CompareInt` _returnvalue 3
    (:`>`
      (`/Engine/EditorBlueprintResources/StandardMacros.CompareInt` _returnvalue 24
        (:`==`
          (bind _returnvalue_2 (`self.DecodeToFloat` _messagebytes))
          (bind _returnvalue_3 (`self.DecodeToFloat` _messagebytes 4))
          (bind _returnvalue_4 (`self.DecodeToFloat` _messagebytes 8))
          (bind _returnvalue_5 (`self.DecodeToFloat` _messagebytes 12))
          (bind _returnvalue_6 (`self.DecodeToFloat` _messagebytes 16))
          (bind _returnvalue_7 (`self.DecodeToFloat` _messagebytes 20))
          (`SceneComponent.K2_SetWorldTransform` (`self.Cube`) (`KismetMathLibrary.MakeTransform` (`KismetMathLibrary.MakeVector` _returnvalue_2 _returnvalue_3 _returnvalue_4) (`KismetMathLibrary.MakeRotator` _returnvalue_5 _returnvalue_6 _returnvalue_7)) false false))))
    (:`==`
      (`SceneComponent.K2_SetWorldTransform` (`self.Cube`) (`KismetMathLibrary.MakeTransform` (`KismetMathLibrary.MakeVector` (`KismetMathLibrary.Conv_ByteToDouble` (`|GetArrayItem` _messagebytes)) (`KismetMathLibrary.Conv_ByteToDouble` (`|GetArrayItem` _messagebytes 1)) (`KismetMathLibrary.Conv_ByteToDouble` (`|GetArrayItem` _messagebytes 2)))) false false)))
  (return true))

(fn `UserConstructionScript`)