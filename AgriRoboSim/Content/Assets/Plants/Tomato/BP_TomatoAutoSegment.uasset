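; Tomato plant actor that picks a plant variant and textures it for either colored or segmentation image generation.
; On BeginPlay it selects a variant from a world-position hash when Randomized, otherwise a fixed one, loading mesh, scale and disease state from TomatoAuto_DT.
; Actor tags choose diffuse or segment textures, applied to leaf and stem slots via dynamic material instances.
; Segment-tagged plants render only in scene captures.
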(event `self.ReceiveBeginPlay`
  (bind (_returnvalue_x _returnvalue_y) (`KismetMathLibrary.BreakVector` (`SceneComponent.K2_GetComponentLocation` (`self.PlantMesh`))))
  (if (`self.Randomized`)
    (`self.ChangePlant` (`KismetMathLibrary.Clamp` (`KismetMathLibrary.FTrunc` (* (+ (`KismetMathLibrary.Cos` (* (`KismetMathLibrary.DegSin` _returnvalue_x) _returnvalue_y 1.0)) 1.0) 5.0)) 1 10))
    (else
      (`self.ChangePlant` 2))))

(fn `ChangeLeafMaterial`
  (params (Diseased :type Boolean) (Mesh :type "StaticMeshComponent Object Reference") (MaterialIndex :type Integer) (Segment :type Boolean))
  (bind _returnvalue (`KismetMaterialLibrary.CreateDynamicMaterialInstance` (`PrimitiveComponent.GetMaterial` Mesh MaterialIndex)))
  (if Diseased
    (if Segment
      (`MaterialInstanceDynamic.SetTextureParameterValue` _returnvalue "Color" "/Game/Tomatos/modified/tomato_plantation_MAX01/Textures/tomato_plants_segment_disease_med.tomato_plants_segment_disease_med")
      (else
        (`MaterialInstanceDynamic.SetTextureParameterValue` _returnvalue "Color" "/Game/Tomatos/modified/tomato_plantation_MAX01/Textures/tomato_plants_defuse_disease_med.tomato_plants_defuse_disease_med")))
    (elif Segment
      (`MaterialInstanceDynamic.SetTextureParameterValue` _returnvalue "Color" "/Game/Assets/Textures/Unlit_Plant_T.Unlit_Plant_T")
      (else
        (`MaterialInstanceDynamic.SetTextureParameterValue` _returnvalue "Color" "/Game/Tomatos/modified/tomato_plantation_MAX01/Textures/tomato_plants_defuse_2_199978_Tex.tomato_plants_defuse_2_199978_Tex"))))
  (`PrimitiveComponent.SetMaterial` Mesh MaterialIndex _returnvalue))

(fn `ChangePlant`
  (params (PlantSelection :type Integer))
  (returns (PlantName :type String))
  (locals (NewLocalVar :type "StaticMaterial Structure"))
  (bind _plantmesh (`self.PlantMesh`))
  (bind _plantmesh_2 (`self.PlantMesh`))
  (`KismetSystemLibrary.PrintString` "Change Plant")
  (bind _returnvalue (`|GetDataTableRow` "/Game/Assets/Plants/Tomato/TomatoAuto_DT.TomatoAuto_DT" (`KismetStringLibrary.Conv_StringToName` (`KismetStringLibrary.Conv_IntToString` PlantSelection)))
    (:`then`
      (bind _output (`|ConvertAsset` (`.Mesh_21_C61ED59E4333D2C6C8B34985FFF4948E` (break `/Game/Assets/Plants/Tomato/TomatoAuto_S` _returnvalue))))
      (`StaticMeshComponent.SetStaticMesh` (`self.MeshHold`) _output)
      (`StaticMeshComponent.SetStaticMesh` _plantmesh _output)
      (`SceneComponent.SetWorldScale3D` _plantmesh (`KismetMathLibrary.Conv_DoubleToVector` (break `/Game/Assets/Plants/Tomato/TomatoAuto_S` _returnvalue)))
      (if (`self.ActorHasTag` "ColoredImageGen")
        (`self.ChangeLeafMaterial` (`.Diseased_25_479F402C46F6BF77DDFC65A53C899EBD` (break `/Game/Assets/Plants/Tomato/TomatoAuto_S` _returnvalue)) _plantmesh_2 (`.LeafMaterialIndex_28_0C94A8E94EDF7F6B6DD72AB572A64DB0` (break `/Game/Assets/Plants/Tomato/TomatoAuto_S` _returnvalue)))
        (bind _returnvalue_2 (- 1 (`.LeafMaterialIndex_28_0C94A8E94EDF7F6B6DD72AB572A64DB0` (break `/Game/Assets/Plants/Tomato/TomatoAuto_S` _returnvalue))))
        (`self.ChangeStemMaterial` _plantmesh_2 _returnvalue_2)
        (return (`KismetTextLibrary.Conv_TextToString` (`.Name_7_5C4A3A3245FEDBE223E9DFBD058681B7` (break `/Game/Assets/Plants/Tomato/TomatoAuto_S` _returnvalue))))
        (elif (`self.ActorHasTag` "SegmentImageGen")
          (`PrimitiveComponent.SetVisibleInSceneCaptureOnly` _plantmesh_2 true)
          (`self.ChangeLeafMaterial` (`.Diseased_25_479F402C46F6BF77DDFC65A53C899EBD` (break `/Game/Assets/Plants/Tomato/TomatoAuto_S` _returnvalue)) _plantmesh_2 (`.LeafMaterialIndex_28_0C94A8E94EDF7F6B6DD72AB572A64DB0` (break `/Game/Assets/Plants/Tomato/TomatoAuto_S` _returnvalue)) true)
          (`self.ChangeStemMaterial` _plantmesh_2 _returnvalue_2 true)
          (return (`KismetTextLibrary.Conv_TextToString` (`.Name_7_5C4A3A3245FEDBE223E9DFBD058681B7` (break `/Game/Assets/Plants/Tomato/TomatoAuto_S` _returnvalue))))
          (else
            (`KismetSystemLibrary.PrintString` "Please Assign a valid tag to BP_TomatoAutoSegment")))))
    (:`RowNotFound`
      (`KismetSystemLibrary.PrintString` "No Row Found" true true (struct :`R` 1.0 :`B` 0.07037 :`A` 1.0))
      (return "PlantNotFound"))))

(fn `ChangeStemMaterial`
  (params (Mesh :type "StaticMeshComponent Object Reference") (MaterialIndex :type Integer) (Segment :type Boolean))
  (bind _returnvalue (`KismetMaterialLibrary.CreateDynamicMaterialInstance` (`PrimitiveComponent.GetMaterial` Mesh MaterialIndex)))
  (if Segment
    (`MaterialInstanceDynamic.SetTextureParameterValue` _returnvalue "Color" "/Game/Tomatos/modified/tomato_plantation_MAX01/Textures/tomato_stems_segment.tomato_stems_segment")
    (else
      (`MaterialInstanceDynamic.SetTextureParameterValue` _returnvalue "Color" "/Game/Tomatos/modified/tomato_plantation_MAX01/Textures/Tomato_stems_defuse_2_2_Tex.Tomato_stems_defuse_2_2_Tex")))
  (`PrimitiveComponent.SetMaterial` Mesh MaterialIndex _returnvalue))

(fn `UserConstructionScript`)