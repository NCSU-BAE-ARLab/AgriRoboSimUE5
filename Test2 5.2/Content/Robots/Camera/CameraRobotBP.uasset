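; Camera robot Blueprint that moves its Cube component from messages received through a game server connection.
; It connects to the game server on BeginPlay, and its message-processing override handles messages exactly three bytes long.
; Each byte becomes one world-space X, Y or Z coordinate for the Cube, and the handler then returns true.
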(event `self.ReceiveBeginPlay`
  (`self.ConnectToGameServer`))

(fn `MessageProcessImplementableEvent`
  (returns (ReturnValue :type Boolean))
  (locals (NewLocalVar :type "Array of Byte"))
  (bind _messagebytes (`self.MessageBytes`))
  (`/Engine/EditorBlueprintResources/StandardMacros.CompareInt` (`KismetArrayLibrary.Array_Length` _messagebytes) 3
    (:`==`
      (`SceneComponent.K2_SetWorldLocation` (`self.Cube`) (`KismetMathLibrary.MakeVector` (`KismetMathLibrary.Conv_ByteToDouble` (`|GetArrayItem` _messagebytes)) (`KismetMathLibrary.Conv_ByteToDouble` (`|GetArrayItem` _messagebytes 1)) (`KismetMathLibrary.Conv_ByteToDouble` (`|GetArrayItem` _messagebytes 2))) false false)
      (return true))))

(fn `UserConstructionScript`)