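; UR10 robot arm actor with a camera rig that generates color, segmentation and depth image datasets.
; Tick drives six physics-constraint joints from ROS vectors or default inputs and records end-effector position.
; A camera line trace passes hit UVs to plants or cylinders as seen areas.
; While TakeData is set, scene captures render on successive frames; clearing it exports PNG/EXR images and logs camera poses to CSV.
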(event `self.ReceiveBeginPlay`
  (bind _datacapturescene2d (`self.DataCaptureScene2D`))
  (bind _segmcapturescene2d (`self.SegmCaptureScene2d`))
  (bind _robotcam_ideal_ (`self.RobotCam(Ideal)`))
  (bind _depthcapturescene2d (`self.DepthCaptureScene2D`))
  (bind _cinecamera (`self.CineCamera`))
  (bind _motorstrength (`self.MotorStrength`))
  (set `self.MotorRatio` 35.0)
  (bind _output_get (set `self.MotorStrength` 10000.0))
  (`PhysicsConstraintComponent.SetAngularDriveParams` (`self.joint4`) (* (`self.MotorRatio`) _motorstrength 0.6) _output_get 0.0)
  (`PhysicsConstraintComponent.SetAngularDriveParams` (`self.joint5`) (* (`self.MotorRatio`) _motorstrength 0.6) _output_get 0.0)
  (`PhysicsConstraintComponent.SetAngularDriveParams` (`self.joint6`) (* (`self.MotorRatio`) _motorstrength 0.6) _output_get 0.0)
  (`PhysicsConstraintComponent.SetAngularDriveParams` (`self.joint1`) (* (`self.MotorRatio`) _motorstrength 1.0) _motorstrength 1000.0)
  (`PhysicsConstraintComponent.SetAngularDriveParams` (`self.joint2`) (* (`self.MotorRatio`) _motorstrength 1.0) _motorstrength 1000.0)
  (`PhysicsConstraintComponent.SetAngularDriveParams` (`self.joint3`) (* (`self.MotorRatio`) _motorstrength 0.8) _motorstrength 0.0)
  (if (`self.Cinecam`)
    (`self.CameraSceneCompStartup` _cinecamera _datacapturescene2d _segmcapturescene2d _depthcapturescene2d)
    (`ActorComponent.Activate` _cinecamera false)
    (else
      (`self.CameraSceneCompStartup` _robotcam_ideal_ _datacapturescene2d _segmcapturescene2d _depthcapturescene2d)
      (`ActorComponent.Activate` _robotcam_ideal_ false))))

(event `self.ReceiveTick`
  (params (DeltaSeconds :type "Float (single-precision)"))
  (bind _readytosave (`self.ReadyToSave`))
  ;[1 1 1] MainLoop
  (`self.CountTime_Event` DeltaSeconds (`self.CycleTimeConst`))
  (if (`self.UseROS`)
    (`self.UseROSInputs_Event` (`self.ArmID`))
    (else
      (`self.DefaultInputs_Event` (`self.CountTimeTrigger`))))
  (`self.UpdateArmPosition_Event`)
  (`self.DrawSeenPlant`)
  (`self.CheckArmPosition_Event`)
  (if (`self.takeData`)
    (if _readytosave
      (`/Engine/EditorBlueprintResources/StandardMacros.CompareInt` (`self.SceneCapID`) 1
        (:`>`
          (`SceneCaptureComponent2D.CaptureScene` (`self.SegmCaptureScene2d`))
          (set `self.SceneCapID` 0)
          (`KismetSystemLibrary.PrintString` "All Rendered"))
        (:`==`
          (`SceneCaptureComponent2D.CaptureScene` (`self.DataCaptureScene2D`))
          (set `self.SceneCapID` (+ (`self.SceneCapID`) 1) :!label _label))
        (:`<`
          (`SceneCaptureComponent2D.CaptureScene` (`self.DepthCaptureScene2D`))
          (goto _label)))
      (else
        (set `self.ReadyToSave` true)
        (set `self.SceneCapID` 0)
        (`PrimitiveComponent.SetSimulatePhysics` (`self.NONE_SAFE_7`) false)))
    (elif _readytosave
      (set `self.ReadyToSave` false)
      (`self.TakeData_Event` (`self.DataCaptureScene2D`) "Color")
      (`self.TakeData_Event` (`self.SegmCaptureScene2d`) "Segment")
      (`self.TakeData_Event` (`self.DepthCaptureScene2D`) "Depth" true)
      (`KismetSystemLibrary.PrintString` "Done")
      (`PrimitiveComponent.SetSimulatePhysics` (`self.NONE_SAFE_7`) true))))

(event `RGBDataEvent`
  (params (bSuccess :type Boolean))
  (`KismetSystemLibrary.PrintString` (`KismetStringLibrary.Conv_BoolToString` bSuccess))
  (if bSuccess
    (`KismetSystemLibrary.PrintString` (`KismetStringLibrary.Concat_StrStr` (`KismetStringLibrary.Concat_StrStr` (`KismetSystemLibrary.GetProjectSavedDirectory`) "Test//temp") "/" (`KismetStringLibrary.Concat_StrStr` (`KismetStringLibrary.Conv_IntToString` (`self.ArmID`)) "_" (`KismetStringLibrary.Conv_IntToString` (+ (`self.ImageCount`) 1)) "_" (stale `TakeData_Event` ImgType) ".exr")))))

(event `CheckArmPosition_Event`
  ;[1 1 1] Get World Position of the last joint (for publish in ROS)
  (set `self.eefJointPos` (`SceneComponent.K2_GetComponentLocation` (`self.EEF`))))

(event `UseROSInputs_Event`
  (params (ID :type Integer))
  ;[1 1 1] ROS Vec3 Inputs to set joint angles
  (set `self.Joint1Rotator` (`KismetMathLibrary.MakeRotator` 0.0 (.x (`self.firstSet`))))
  (set `self.Joint2Roator` (`KismetMathLibrary.MakeRotator` 0.0 0.0 (.y (`self.firstSet`))))
  (set `self.Joint3Rotator` (`KismetMathLibrary.MakeRotator` 0.0 0.0 (.z (`self.firstSet`))))
  (set `self.Joint4Rotator` (`KismetMathLibrary.MakeRotator` 0.0 0.0 (.x (`self.secondSet`))))
  (set `self.Joint5Rotator` (`KismetMathLibrary.MakeRotator` 0.0 (.y (`self.secondSet`))))
  (set `self.Joint6Rotator` (`KismetMathLibrary.MakeRotator` 0.0 0.0 (.z (`self.secondSet`)))))

(event `TakeData_Event`
  (params (SceneCap2d :type "SceneCaptureComponent2D Object Reference") (ImgType :type String) (`HDR(Depth)` :type Boolean))
  (bind _texturetarget (`SceneCaptureComponent2D.TextureTarget` SceneCap2d))
  (bind _camlocationarr (`self.CamLocationArr`))
  (bind _returnvalue (`KismetStringLibrary.Conv_IntToString` (`self.ArmID`)))
  (bind (_x _y _z) (`KismetMathLibrary.BreakVector3f` (`SceneComponent.K2_GetComponentLocation` SceneCap2d)))
  (bind _returnvalue_2 (`KismetStringLibrary.Concat_StrStr` (`KismetSystemLibrary.GetProjectSavedDirectory`) "Test//temp"))
  (bind _returnvalue_3 (+ (`self.ImageCount`) 1))
  (bind (_x_2 _y_2 _z_2 _w) (`KismetMathLibrary.BreakQuat` (`KismetMathLibrary.Conv_RotatorToQuaternion` (`SceneComponent.K2_GetComponentRotation` SceneCap2d))))
  (bind _returnvalue_4 (`KismetStringLibrary.Concat_StrStr` _returnvalue_2 "/" (`KismetStringLibrary.Concat_StrStr` _returnvalue "_" (`KismetStringLibrary.Conv_IntToString` _returnvalue_3) "_" ImgType ".exr")))
  ;[1 1 1] Generate Image and Text Data
  (if `HDR(Depth)`
    (`ImageWriteBlueprintLibrary.ExportToDisk` _texturetarget _returnvalue_4 (make `ImageWriteOptions` "EXR" (`|CreateDelegate` :!event `RGBDataEvent`)))
    (else
      (`ImageWriteBlueprintLibrary.ExportToDisk` _texturetarget _returnvalue_4 (make `ImageWriteOptions` "PNG" (`|CreateDelegate` :!event `RGBDataEvent`)))))
  (set `self.ImageCount` _returnvalue_3)
  (`KismetArrayLibrary.Array_Append` _camlocationarr (`|MakeArray` (`KismetStringLibrary.BuildString_Int` (`KismetStringLibrary.BuildString_Int` (`KismetStringLibrary.BuildString_Double` (`KismetStringLibrary.BuildString_Double` (`KismetStringLibrary.BuildString_Double` (`KismetStringLibrary.BuildString_Double` (`KismetStringLibrary.BuildString_Double` (`KismetStringLibrary.BuildString_Double` (`KismetStringLibrary.BuildString_Double` ImgType "," _x ",") "" _y ",") "" _z ",") "" _x_2 ",") "" _y_2 ",") "" _z_2 ",") "" _w ",") "" (`self.ArmID`) ",") "" (`self.ImageCount`) ",")))
  (`self.saveCamData` (`KismetStringLibrary.Concat_StrStr` _returnvalue_2 "//" _returnvalue "camLocation.csv") _camlocationarr))

(event `DefaultInputs_Event`
  (params (RandomVal :type "Boolean (by ref)"))
  (bind _randomval (`self.RandomVal`))
  ;[1 1 1] Default Inputs to set joint angles
  (if RandomVal
    (set `self.RandomVal` 180.0))
  (set `self.Joint1Rotator` (`KismetMathLibrary.MakeRotator` 0.0 _randomval))
  (set `self.Joint2Roator` (`KismetMathLibrary.MakeRotator` 0.0 0.0 _randomval))
  (set `self.Joint3Rotator` (`KismetMathLibrary.MakeRotator` 0.0 0.0 _randomval))
  (set `self.Joint4Rotator` (`KismetMathLibrary.MakeRotator` 0.0 0.0 _randomval))
  (set `self.Joint5Rotator` (`KismetMathLibrary.MakeRotator` 0.0 _randomval))
  (set `self.Joint6Rotator` (`KismetMathLibrary.MakeRotator` 0.0 0.0 _randomval))
  (`KismetSystemLibrary.PrintString` (`KismetStringLibrary.Conv_DoubleToString` _randomval) false false))

(event `UpdateArmPosition_Event`
  ;[1 1 1] UpdateArmPosition
  (`PhysicsConstraintComponent.SetAngularOrientationTarget` (`self.joint1`) (`self.Joint1Rotator`))
  (`PhysicsConstraintComponent.SetAngularOrientationTarget` (`self.joint2`) (`self.Joint2Roator`))
  (`PhysicsConstraintComponent.SetAngularOrientationTarget` (`self.joint3`) (`self.Joint3Rotator`))
  (`PhysicsConstraintComponent.SetAngularOrientationTarget` (`self.joint4`) (`self.Joint4Rotator`))
  (`PhysicsConstraintComponent.SetAngularOrientationTarget` (`self.joint5`) (`self.Joint5Rotator`))
  (`PhysicsConstraintComponent.SetAngularOrientationTarget` (`self.joint6`) (`self.Joint6Rotator`)))

(event `CountTime_Event`
  (params (DeltaSeconds :type "Float (double-precision) (by ref)") (CountSeconds :type "Float (double-precision) (by ref)"))
  (bind _cycletime (`self.CycleTime`))
  (bind _returnvalue (+ DeltaSeconds _cycletime))
  (bind _returnvalue_2 (> _returnvalue CountSeconds))
  ;[1 1 1] Time Trigger Once
  (set `self.CycleTime` _returnvalue)
  (set `self.CountTimeTrigger` _returnvalue_2)
  (if _returnvalue_2
    (set `self.CycleTime` (- _cycletime CountSeconds -1.0))))

(fn `CameraSceneCompStartup`
  (params (`Camera Settings` :type "CameraComponent Object Reference") (`Colored SceneCap` :type "SceneCaptureComponent2D Object Reference") (`Segmentation SceneCap` :type "SceneCaptureComponent2D Object Reference") (`Depth SceneCap` :type "SceneCaptureComponent2D Object Reference"))
  (bind _desiredview (`CameraComponent.GetCameraView` `Camera Settings` 0.0))
  (bind (_location _rotation _fov _orthowidth _orthonearclipplane _orthofarclipplane _perspectivenearclipplane _aspectratio _bconstrainaspectratio _busefieldofviewforlod _projectionmode _postprocessblendweight _postprocesssettings) (break `MinimalViewInfo` _desiredview))
  ;[1 1 1] Depth
  (bind _output_get (set `SceneCaptureComponent2D.FOVAngle` _fov `Depth SceneCap`))
  ;[1 1 1] Segmentation
  (bind _output_get_2 (set `SceneCaptureComponent2D.FOVAngle` _output_get `Segmentation SceneCap`))
  ;[1 1 1] Colored
  (set `SceneCaptureComponent2D.FOVAngle` _output_get_2 `Colored SceneCap`)
  (bind _output_get_3 (set `SceneCaptureComponent2D.ProjectionType` _projectionmode `Depth SceneCap`))
  (bind _output_get_4 (set `SceneCaptureComponent2D.ProjectionType` _output_get_3 `Segmentation SceneCap`))
  (set `SceneCaptureComponent2D.ProjectionType` _output_get_4 `Colored SceneCap`)
  (bind _output_get_5 (set `SceneCaptureComponent2D.PostProcessBlendWeight` _postprocessblendweight `Depth SceneCap`))
  (bind _output_get_6 (set `SceneCaptureComponent2D.PostProcessBlendWeight` _output_get_5 `Segmentation SceneCap`))
  (set `SceneCaptureComponent2D.PostProcessBlendWeight` _output_get_6 `Colored SceneCap`)
  (bind _output_get_7 (set `SceneCaptureComponent2D.PostProcessSettings` _postprocesssettings `Depth SceneCap`))
  (bind _output_get_8 (set `SceneCaptureComponent2D.PostProcessSettings` _output_get_7 `Segmentation SceneCap`))
  (set `SceneCaptureComponent2D.PostProcessSettings` _output_get_8 `Colored SceneCap`)
  (bind _outactors (`GameplayStatics.GetAllActorsWithTag` "ColoredImageGen"))
  (bind _outactors_2 (`GameplayStatics.GetAllActorsWithTag` "SegmentImageGen"))
  (bind _outactors_3 (`GameplayStatics.GetAllActorsWithTag` "ColoredImageGen"))
  (set `SceneCaptureComponent.ShowOnlyActors` _outactors `Depth SceneCap`)
  (set `SceneCaptureComponent.ShowOnlyActors` _outactors_2 `Segmentation SceneCap`)
  (set `SceneCaptureComponent.ShowOnlyActors` _outactors_3 `Colored SceneCap`)
  (`self.Refresh RT` `Depth SceneCap` true)
  (`self.Refresh RT` `Segmentation SceneCap`)
  (`self.Refresh RT` `Colored SceneCap`))

(fn `DrawSeenPlant`
  (bind _robotcam_ideal_ (`self.RobotCam(Ideal)`))
  (bind _returnvalue (`SceneComponent.K2_GetComponentLocation` _robotcam_ideal_))
  (bind (_outhit _returnvalue_2) (`KismetSystemLibrary.LineTraceSingle` _returnvalue (+ _returnvalue (* (`SceneComponent.GetForwardVector` _robotcam_ideal_) 200.0)) "TraceTypeQuery2"))
  (if _returnvalue_2
    (bind (_bblockinghit _binitialoverlap _time _distance _location _impactpoint _normal _impactnormal _physmat _hitactor) (`GameplayStatics.BreakHitResult` _outhit))
    (bind _asbp_plant (cast `/Game/Assets/Painting/BP_Plant` _hitactor)
      (:`then`
        (bind _uv (`GameplayStatics.FindCollisionUV` _outhit))
        (`/Game/Assets/Painting/BP_Plant.SeenArea` _asbp_plant _uv))
      (:`CastFailed`
        (bind _asbp_cylinder (cast `/Game/Assets/Painting/BP_Cylinder` _hitactor))
        (`/Game/Assets/Painting/BP_Cylinder.SeenArea` _asbp_cylinder _uv)))))

(fn `Refresh RT`
  (params (SceneCap2D :type "SceneCaptureComponent2D Object Reference") (SceneDepth :type Boolean :default false))
  (if SceneDepth
    (bind _returnvalue (`KismetRenderingLibrary.CreateRenderTarget2D` 1920 1080 "RTF_RGBA32f"))
    (set `TextureRenderTarget.TargetGamma` 2.5 _returnvalue)
    (bind _output_get (set `self.camImage` _returnvalue))
    (bind _output_get_2 (set `SceneCaptureComponent2D.TextureTarget` _output_get SceneCap2D))
    (else
      (bind _returnvalue_2 (`KismetRenderingLibrary.CreateRenderTarget2D` 1920 1080 "RTF_RGBA8_SRGB"))
      (set `TextureRenderTarget.TargetGamma` 2.5 _returnvalue_2)
      (bind _output_get_3 (set `self.camImage` _returnvalue_2))
      (bind _output_get_4 (set `SceneCaptureComponent2D.TextureTarget` _output_get_3 SceneCap2D)))))

(fn `UserConstructionScript`)