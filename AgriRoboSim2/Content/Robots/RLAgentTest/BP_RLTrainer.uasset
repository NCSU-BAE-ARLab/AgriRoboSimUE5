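; BP_RLTrainer is a Learning Agents trainer that defines rewards, completion and episode resets for BP_Agent in an RL test.
; Reward combines location similarity, logged to the Visual Logger, with a bonus within a small distance threshold of the default target location.
; The proximity completion check uses type Running, so reaching the target does not end the episode.
; Episode reset moves the agent to a random location.
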(fn `GatherAgentCompletion`
  (params (AgentId :type Integer))
  (returns (OutCompletion :type "ELearningAgentsCompletion Enum"))
  (return (`LearningAgentsCompletions.MakeCompletionOnLocationDifferenceBelowThreshold` (`Actor.K2_GetActorLocation` (`self.GetAgent` AgentId "/Game/Robots/RLAgentTest/BP_Agent.BP_Agent_C")) (0.0 0.0 0.0) 10.0 "Running" "LocationDifferenceBelowThresholdCompletion" false null)))

(fn `GatherAgentReward`
  (params (AgentId :type Integer))
  (returns (OutReward :type "Float (single-precision)"))
  (locals (RewardActor :type "/Game/Robots/RLAgentTest/BP_Agent Object Reference"))
  (bind _returnvalue_location (`KismetMathLibrary.BreakTransform` (`Actor.GetTransform` (`local.RewardActor`))))
  (set `local.RewardActor` (`self.GetAgent` AgentId "/Game/Robots/RLAgentTest/BP_Agent.BP_Agent_C"))
  (return (+ (`LearningAgentsRewards.MakeRewardFromLocationSimilarity` _returnvalue_location (0.0 0.0 0.0) 1000.0 1.0 "LocationSimilarityReward" true null AgentId _returnvalue_location) (`LearningAgentsRewards.MakeRewardOnLocationDifferenceBelowThreshold` _returnvalue_location (0.0 0.0 0.0) 10.0 10.0 "LocationDifferenceBelowThresholdReward" false null))))

(fn `ResetAgentEpisode`
  (params (AgentId :type Integer))
  (`/Game/Robots/RLAgentTest/BP_Agent.ResetToRandomLocation` (`self.GetAgent` AgentId "/Game/Robots/RLAgentTest/BP_Agent.BP_Agent_C")))