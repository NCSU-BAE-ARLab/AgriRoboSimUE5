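; Learning Agents interactor that defines what a BP_Agent robot observes and how it acts for reinforcement learning.
; Observations are a struct of location and rotation, passing the agent's transform only as the relative frame, with the observed values left at defaults.
; Actions are a struct of Throttle and Steering floats, written straight to the agent's Throttle and Steer variables.
; Observation and action calls feed the visual logger for debugging.
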(fn `GatherAgentObservation`
  (params (InObservationObject :type "LearningAgentsObservationObject Object Reference") (AgentId :type Integer))
  (returns (OutObservationObjectElement :type "LearningAgentsObservationObjectElement Structure"))
  (bind _returnvalue (`self.GetAgent` AgentId "/Game/Robots/RLAgentTest/BP_Agent.BP_Agent_C"))
  (bind _returnvalue_2 (`Actor.K2_GetActorLocation` _returnvalue))
  (return (`LearningAgentsObservations.MakeStructObservation` InObservationObject (`|MakeMap` "Location" (`LearningAgentsObservations.MakeLocationObservation` InObservationObject (0.0 0.0 0.0) (`Actor.GetTransform` _returnvalue) 1000.0 "LocationObservation" false null AgentId _returnvalue_2) "Direction" (`LearningAgentsObservations.MakeRotationObservation` InObservationObject (struct) (`Actor.K2_GetActorRotation` _returnvalue) "RotationObservation" false null AgentId _returnvalue_2 _returnvalue_2) :!type "Name"))))

(fn `PerformAgentAction`
  (params (InActionObject :type "LearningAgentsActionObject Object Reference") (InActionObjectElement :type "LearningAgentsActionObjectElement Structure (by ref)") (AgentId :type Integer))
  (locals (ActActor :type "/Game/Robots/RLAgentTest/BP_Agent Object Reference"))
  (bind _inactionobject (`local.InActionObject`))
  (bind _actactor (`local.ActActor`))
  (bind _output_get (set `local.ActActor` (`self.GetAgent` AgentId "/Game/Robots/RLAgentTest/BP_Agent.BP_Agent_C")))
  (bind _outelements (`LearningAgentsActions.GetStructAction` InActionObject InActionObjectElement))
  (`|ExecutionSequence`
    (:`then_0`
      (bind _returnvalue (`Actor.K2_GetActorLocation` _output_get))
      (bind _outvalue (`LearningAgentsActions.GetFloatAction` _inactionobject (`BlueprintMapLibrary.Map_Find` _outelements "Steering") 1.0 "Steering" false null AgentId _returnvalue))
      (set `/Game/Robots/RLAgentTest/BP_Agent.Steer` _outvalue _actactor))
    (:`then_1`
      (bind _outvalue_2 (`LearningAgentsActions.GetFloatAction` _inactionobject (`BlueprintMapLibrary.Map_Find` _outelements "Throttle") 1.0 "Throttle" false null AgentId _returnvalue))
      (set `/Game/Robots/RLAgentTest/BP_Agent.Throttle` _outvalue_2 _actactor))
    (:`then_2`
      (return))))

(fn `SpecifyAgentAction`
  (params (InActionSchema :type "LearningAgentsActionSchema Object Reference"))
  (returns (OutActionSchemaElement :type "LearningAgentsActionSchemaElement Structure"))
  (return (`LearningAgentsActions.SpecifyStructAction` InActionSchema (`|MakeMap` "Throttle" (`LearningAgentsActions.SpecifyFloatAction` InActionSchema "Throttle") "Steering" (`LearningAgentsActions.SpecifyFloatAction` InActionSchema "Steering") :!type "Name"))))

(fn `SpecifyAgentObservation`
  (params (InObservationSchema :type "LearningAgentsObservationSchema Object Reference"))
  (returns (OutObservationSchemaElement :type "LearningAgentsObservationSchemaElement Structure"))
  (return (`LearningAgentsObservations.SpecifyStructObservation` InObservationSchema (`|MakeMap` "Location" (`LearningAgentsObservations.SpecifyLocationObservation` InObservationSchema) "Direction" (`LearningAgentsObservations.SpecifyRotationObservation` InObservationSchema) :!type "Name"))))