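; BP_Agent is a simple cube agent that Learning Agents managers control in a reinforcement learning test.
; On BeginPlay it registers itself with every tagged actor holding a LearningAgentsManager component, printing a warning if none is found.
; Each tick it moves the cube forward by clamped Throttle and yaws it by Steer.
; ResetToRandomLocation teleports the cube to a random ground-plane position and yaw.
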(event `self.ReceiveBeginPlay`
  (bind _outactors (`GameplayStatics.GetAllActorsWithTag` "LearningAgentsManager"))
  (for _array_element _outactors
    (bind _returnvalue (`self.GetComponentByClass` _array_element "/Script/LearningAgents.LearningAgentsManager"))
    (`/Engine/EditorBlueprintResources/StandardMacros.IsValid` _returnvalue
      (:`Is Valid`
        (`LearningAgentsManager.AddAgent` _returnvalue self)
        (set `self.FoundManager` true))))
  (if (not (`self.FoundManager`))
    (`KismetSystemLibrary.PrintString` "No Learning Manager Found")))

(event `self.ReceiveTick`
  (params (DeltaSeconds :type "Float (single-precision)"))
  (`SceneComponent.K2_AddRelativeLocation` (`self.Cube`) (* (`SceneComponent.GetForwardVector` (`self.Cube`)) (`KismetMathLibrary.FClamp` (`self.Throttle`) -1.0 3.0)) false false)
  (`SceneComponent.K2_AddLocalRotation` (`self.Cube`) (`KismetMathLibrary.MakeRotator` 0.0 0.0 (* (`self.Steer`) 10.0)) false false))

(fn `ResetToRandomLocation`
  (`SceneComponent.K2_SetWorldLocationAndRotation` (`self.Cube`) (`KismetMathLibrary.MakeVector` (`KismetMathLibrary.RandomFloatInRange` -1000.0 1000.0) (`KismetMathLibrary.RandomFloatInRange` -1000.0 1000.0)) (`KismetMathLibrary.MakeRotator` 0.0 0.0 (`KismetMathLibrary.RandomFloatInRange` -1000.0 1000.0)) false true))

(fn `UserConstructionScript`)