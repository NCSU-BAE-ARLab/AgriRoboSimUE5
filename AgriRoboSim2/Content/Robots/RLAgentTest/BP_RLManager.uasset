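; BP_RLManager is a Learning Agents reinforcement learning manager that trains or runs a learned policy for BP_Agent actors.
; BeginPlay makes itself their tick prerequisite, then chains interactor, policy, critic and trainer creation, using existing neural network assets without reinitializing them.
; A RunInference flag switches Tick between policy inference and training.
; In inference mode, BeginPlay also resets agents to random locations.
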(event `self.ReceiveBeginPlay`
  (`|ExecutionSequence`
    (:`then_0`
      (bind _outactors (`GameplayStatics.GetAllActorsOfClass` "/Game/Robots/RLAgentTest/BP_Agent.BP_Agent_C"))
      (bind _output_get (set `self.AgentActors` _outactors))
      (`self.AddTickPrerequisiteActor` _output_get self))
    (:`then_1`
      (bind _returnvalue (`LearningAgentsInteractor.MakeInteractor` (`self.LearningAgentsManager`) "/Game/Robots/RLAgentTest/BP_RLInteractor.BP_RLInteractor_C"))
      (set `self.Interactor` _returnvalue))
    (:`then_2`
      (bind _returnvalue_2 (`LearningAgentsPolicy.MakePolicy` (`self.LearningAgentsManager`) (`self.Interactor`) "/Script/LearningAgents.LearningAgentsPolicy" "Policy" "/Game/Robots/RLAgentTest/DA_RLEncoder.DA_RLEncoder" "/Game/Robots/RLAgentTest/DA_RLPolicy.DA_RLPolicy" "/Game/Robots/RLAgentTest/DA_RLDecoder.DA_RLDecoder" false false false (`self.Policy Settings`)))
      (set `self.Policy` _returnvalue_2))
    (:`then_3`
      (bind _returnvalue_3 (`LearningAgentsCritic.MakeCritic` (`self.LearningAgentsManager`) (`self.Interactor`) (`self.Policy`) "/Script/LearningAgents.LearningAgentsCritic" "Critic" "/Game/Robots/RLAgentTest/DA_RLCritic.DA_RLCritic" false (`self.Critic Settings`)))
      (set `self.Critic` _returnvalue_3))
    (:`then_4`
      (bind _returnvalue_4 (`LearningAgentsTrainer.MakeTrainer` (`self.LearningAgentsManager`) (`self.Interactor`) (`self.Policy`) (`self.Critic`) "/Game/Robots/RLAgentTest/BP_RLTrainer.BP_RLTrainer_C" "Trainer" (`self.Trainer Settings`)))
      (set `self.Trainer` _returnvalue_4))
    (:`then_5`
      (if (`self.RunInference`)
        (`/Game/Robots/RLAgentTest/BP_Agent.ResetToRandomLocation` (`self.AgentActors`))))))

(event `self.ReceiveTick`
  (params (DeltaSeconds :type "Float (single-precision)"))
  (if (`self.RunInference`)
    (`LearningAgentsPolicy.RunInference` (`self.Policy`) 0.0)
    (else
      (`LearningAgentsTrainer.RunTraining` (`self.Trainer`) (`self.Trainer Training Settings`) (`self.Trainer Game Settings`) (`self.Trainer Path Settings_0`) true true))))

(fn `UserConstructionScript`)