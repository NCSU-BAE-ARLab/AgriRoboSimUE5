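; Data-driven ROS robot actor that simulates a selectable arm with optional cameras and gripper scanning.
; BeginPlay applies mesh, physics and joint profile from a DataTable, spawns SemanticRobot_BP, and attaches HitScanner actors and the end-effector camera to sockets.
; Tick follows any parent robot socket, drives joint targets, publishes robot state and averages gripper hit distances.
; Looping timers capture and publish color, depth and optional stereo or segmentation images to ROS.
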(event `self.ReceiveBeginPlay`
  (bind _joint_topics (`self.Joint Topics`))
  (bind _arm (`self.Arm`))
  (bind _arm_2 (`self.Arm`))
  (bind _cameraparams (`self.CameraParams`))
  (bind _arm_3 (`self.Arm`))
  (bind _rosarmcontrol (`self.ROSArmControl`))
  (bind _roscameracontrol (`self.ROSCameraControl`))
  ;[0.3846 0.6517 1] Robot Swapping
  (bind _returnvalue (`|GetDataTableRow` (`self.RobotSelectionDataTable`) (`self.RobotSelection`))
    (:`then`
      (bind _values (`BlueprintMapLibrary.Map_Values` _joint_topics))
      (set `ROSArmControl.JointNames_ROS` _values _rosarmcontrol)
      (bind _keys (`BlueprintMapLibrary.Map_Keys` _joint_topics))
      (set `ROSArmControl.JointNames_UE` _keys _rosarmcontrol)
      (set `ROSArmControl.bLinearJointType` (`self.B Linear Joint Type`) _rosarmcontrol)
      (bind (_robot _physicsasset _jointprofile _jointbonename _transform _eefsocketname) (break `/Game/Robot/RobotSwap_S` _returnvalue))
      (`SkeletalMeshComponent.SetSkeletalMeshAsset` _arm _robot)
      (`SceneComponent.K2_AddWorldTransform` _arm_2 _transform false true)
      (`SceneComponent.SetWorldScale3D` _arm_2 (.scale _transform))
      (`SkinnedMeshComponent.SetPhysicsAsset` _arm _physicsasset true)
      (`SceneComponent.K2_AttachToComponent` (`self.CineCamera`) (`self.Arm`) _eefsocketname "SnapToTarget" "SnapToTarget" "SnapToTarget" true)
      (`ROSArmControl.InitRobotArm` (`self.ROSArmControl`) (`self.Arm`) _jointprofile _jointbonename (`self.Topic Prefix`))
      (`|SpawnActorFromClass` "/Game/Robot/SemanticRobot_BP.SemanticRobot_BP_C" (`KismetMathLibrary.MakeTransform` (0.0 0.0 0.0)) "Undefined" "MultiplyWithRoot" null self null)
      (`|ExecutionSequence`
        (:`then_0`
          ;[1 1 1] SpawnHitScanInAreaForGripper
          (if (`self.IsGripper`)
            (for _array_element (`self.GripperAttachPoints`)
              (for _array_element_2 (`self.GripperGrids`)
                (bind (_returnvalue_location _returnvalue_rotation _returnvalue_scale) (`KismetMathLibrary.BreakTransform` (`SceneComponent.GetSocketTransform` (`self.Arm`) _array_element "RTS_World")))
                (bind _returnvalue_2 (`|SpawnActorFromClass` "/Game/Robot/HitScan/HitScanner.HitScanner_C" (`KismetMathLibrary.MakeTransform` (+ _returnvalue_location (`KismetMathLibrary.GreaterGreater_VectorRotator` _array_element_2 _returnvalue_rotation)) _returnvalue_rotation _returnvalue_scale) "Undefined" "OverrideRootScale" null 10.0 false null))
                (`self.K2_AttachToComponent` _returnvalue_2 (`self.Arm`) _array_element "KeepWorld" "SnapToTarget" "KeepWorld" true)
                (`KismetArrayLibrary.Array_Add` (`self.ScanLists`) _returnvalue_2)))))
        (:`then_1`
          ;[1 1 1] SpawnHitScan
          (if (`self.HitScanSpawn`)
            (`KismetArrayLibrary.Array_Clear` (`self.HitScan`))
            (for _array_element_3 (`self.HitScanAttachPoints`)
              (if (`SceneComponent.DoesSocketExist` _arm_3 _array_element_3)
                (bind _returnvalue_3 (`|SpawnActorFromClass` "/Game/Robot/HitScan/HitScanner.HitScanner_C" (`SceneComponent.GetSocketTransform` _arm_3 _array_element_3 "RTS_World") "Undefined" "OverrideRootScale" null 10.0 false null))
                (`self.K2_AttachToComponent` _returnvalue_3 _arm_3 _array_element_3 "SnapToTarget" "SnapToTarget" "SnapToTarget" true)
                (`KismetArrayLibrary.Array_Add` (`self.HitScan`) _returnvalue_3)
                (else
                  (`KismetSystemLibrary.PrintString` "SocketDoesNotExistForHitScan"))))))
        (:`then_2`
          ;[1 1 1] Spawn Camera
          (if (`self.HasCamera`)
            (bind _returnvalue_4 (`|GetDataTableRow` _cameraparams (`self.CameraSelection`))
              (:`then`
                (`self.SetCineCamFromDT` _returnvalue_4))
              (:`RowNotFound`
                (bind _returnvalue_5 (`|GetDataTableRow` _cameraparams "Rpiv3W")
                  (:`then`
                    (`self.SetCineCamFromDT` _returnvalue_5)))))
            (set `ROS2NodeComponent.TopicPrefix` (`self.Topic Prefix`) _roscameracontrol)
            (`ROSCameraControl.UpdateFrameIDSources` _roscameracontrol (`self.TrackedObj`))
            (`ROSCameraControl.SetCameraMode` _roscameracontrol "Block")
            (`self.CameraModuleConfig`)
            (`self.CameraTimerConfig` (delegate `PubImage`) (delegate `CaptureTimer`) :!label _label)))))
    (:`RowNotFound`
      (`KismetSystemLibrary.PrintString` "Invalid Robot Selection Name" true true (struct :`G` 0.66 :`B` 1.0 :`A` 1.0) 5.0))))

(event `PubImage`
  (`ROSCameraControl.UpdateAllCameraParameters` (`self.ROSCameraControl`) (`self.CineCamera`))
  (`|ExecutionSequence`
    (:`then_1`
      (`KismetSystemLibrary.DelayUntilNextTick`)
      (if (`self.TogglePub`)
        (`ROSCameraControl.PublishAllTopic` (`self.ROSCameraControl`))))))

(event `CaptureTimer`
  (bind _keys (`BlueprintMapLibrary.Map_Keys` (`self.ActiveCameraMap`)))
  (`SceneCaptureComponent2D.CaptureScene` _keys)
  (`ROSCameraControl.UpdateFrameIDSources` (`self.ROSCameraControl`) (`self.TrackedObj`)))

(event `self.ReceiveTick`
  (params (DeltaSeconds :type "Float (single-precision)"))
  (bind _rosarmcontrol (`self.ROSArmControl`))
  (bind _numhits (`self.NumHits`))
  ;[1 1 1] follow parent socket location
  (`/Engine/EditorBlueprintResources/StandardMacros.IsValid` (`self.ParentRobot`)
    (:`Is Valid`
      (`self.K2_SetActorLocation` (`SceneComponent.GetSocketLocation` (`/Game/Robot/Robot_BP.Arm` (`self.ParentRobot`)) (`self.ParentRobotSocket`)) false true))
    (:`Is Not Valid`
      _))
  ;[1 1 1] Set joint states
  (`ROSArmControl.SetJointsTargets` _rosarmcontrol)
  (`ROSArmControl.PubRobotState` _rosarmcontrol)
  (bind _asmain_game_state_base (cast `/Game/Levels/GameModes/MainMenu/MainGameStateBase` (`GameplayStatics.GetGameState`)))
  (`BlueprintGameplayTagLibrary.AddGameplayTag` (`/Game/Levels/GameModes/MainMenu/MainGameStateBase.ROSSceneInfoGameplayTags` _asmain_game_state_base) (struct :`TagName` "ROSSceneInfo.Period.UpdateInfo"))
  (`|ExecutionSequence`
    (:`then_0`
      (if (`self.HasCamera`)
        (if (`self.CameraUpdate`)
          (`KismetSystemLibrary.K2_ClearAndInvalidateTimerHandle` (`self.CameraTimer`))
          (`ROSCameraControl.InitROSTopics` (`self.ROSCameraControl`) (`self.ActiveCameraMap`) (`self.CineCamera`) (`self.ImageWidth`) (`self.ImageHeight`))
          (set `self.CameraUpdate` false)
          (goto _label))))
    (:`then_1`
      (if (`self.IsGripper`)
        (for _array_element (`self.ScanLists`)
          (if (`|EnumEquality` (`/Game/Robot/HitScan/HitScanner.Tomato Enum` _array_element) "NewEnumerator1")
            (set `self.SumDistanceToHit` (+ (`self.SumDistanceToHit`) (`/Game/Robot/HitScan/HitScanner.DistanceToHit` _array_element)))
            (`/Engine/EditorBlueprintResources/StandardMacros.IncrementInt` (`self.NumHits`))))
        (`TextRenderComponent.K2_SetText` (`self.DebugText`) (`KismetTextLibrary.Conv_StringToText` (`KismetStringLibrary.BuildString_Double` (`KismetStringLibrary.BuildString_Int` "" "Num Hits: " _numhits " ") "Distance: " (/ (`self.SumDistanceToHit`) _numhits))))
        (set `self.NumHits` 0)
        (set `self.SumDistanceToHit` 0.0)))))

(event `ScanHitObject`
  (params (EndLocations :type "Array of Vector Structure"))
  (bind _locationidx (`self.LocationIdx`))
  (`KismetSystemLibrary.PrintString` (`KismetStringLibrary.Conv_IntToString` (`KismetArrayLibrary.Array_Length` EndLocations)))
  (for _array_element (`self.HitScan`)
    (set `/Game/Robot/HitScan/HitScanner.DebugString` "" _array_element)
    (set `/Game/Robot/HitScan/HitScanner.EndLocationPoint` 0 _array_element)
    (`KismetArrayLibrary.Array_Clear` (`/Game/Robot/HitScan/HitScanner.EndLocations` _array_element))
    (`KismetArrayLibrary.Array_Clear` (`/Game/Robot/HitScan/HitScanner.EndLocationsPrefix` _array_element)))
  (bind _output_get (set `self.LocationIdx` 0))
  (if (> (`KismetArrayLibrary.Array_Length` (`self.HitScan`)) 0)
    (bind _returnvalue (< _output_get (`KismetArrayLibrary.Array_Length` EndLocations)))
    (while _returnvalue
      (for _array_element_2 (`self.HitScan`)
        (if _returnvalue
          (`KismetArrayLibrary.Array_Add` (`/Game/Robot/HitScan/HitScanner.EndLocations` _array_element_2) (`|GetArrayItem` EndLocations _locationidx))
          (`KismetArrayLibrary.Array_Add` (`/Game/Robot/HitScan/HitScanner.EndLocationsPrefix` _array_element_2) (`KismetStringLibrary.Conv_IntToString` _locationidx))
          (`/Engine/EditorBlueprintResources/StandardMacros.IncrementInt` _locationidx))))
    (else
      (`KismetSystemLibrary.PrintString` "NoHitScanActors"))))

(fn `CameraModuleConfig`
  (bind _returnvalue (enumliteral `ECaptureType` "ColorCapture"))
  (bind _returnvalue_2 (enumliteral `ECaptureType` "SegmentationCapture"))
  (bind _returnvalue_3 (enumliteral `ECaptureType` "DepthCapture"))
  (bind _issegmentationmode (`self.IsSegmentationMode`))
  (bind _activecameramap (`self.ActiveCameraMap`))
  (`BlueprintMapLibrary.Map_Clear` _activecameramap)
  (`BlueprintMapLibrary.Map_Add` _activecameramap (`self.Color`) _returnvalue)
  (`BlueprintMapLibrary.Map_Add` _activecameramap (`self.Depth`) _returnvalue_3)
  (if (`self.IsStereoMode`)
    (`BlueprintMapLibrary.Map_Add` _activecameramap (`self.ColorOne`) _returnvalue)
    (`BlueprintMapLibrary.Map_Add` _activecameramap (`self.DepthOne`) _returnvalue_3)
    (if _issegmentationmode
      (`BlueprintMapLibrary.Map_Add` _activecameramap (`self.SegmentationOne`) _returnvalue_2)
      (`BlueprintMapLibrary.Map_Add` _activecameramap (`self.Segmentation`) _returnvalue_2))
    (elif _issegmentationmode
      (`BlueprintMapLibrary.Map_Add` _activecameramap (`self.Segmentation`) _returnvalue_2)))
  (set `self.CameraUpdate` true))

(fn `CameraTimerConfig`
  (params (PubTimer :type Delegate) (RenderTimer :type Delegate))
  (bind _imagemessageperiod (`self.ImageMessagePeriod`))
  (if (not (`KismetSystemLibrary.K2_IsTimerActiveHandle` (`self.CameraTimer`)))
    (bind _returnvalue (`KismetSystemLibrary.K2_SetTimerDelegate` PubTimer _imagemessageperiod true true 0.01))
    (set `self.CameraTimer` _returnvalue))
  (if (not (`KismetSystemLibrary.K2_IsTimerActiveHandle` (`self.RenderTimer`)))
    (bind _returnvalue_2 (`KismetSystemLibrary.K2_SetTimerDelegate` RenderTimer (/ _imagemessageperiod 1.0) true true 0.01))
    (set `self.RenderTimer` _returnvalue_2)))

(fn `GetHitObject`)

(fn `GetRobotInfo`
  (returns (Information :type String))
  (bind _returnvalue (`SceneComponent.K2_GetComponentToWorld` (`self.Color`)))
  (bind (_returnvalue_x _returnvalue_y _returnvalue_z _returnvalue_w) (`KismetMathLibrary.BreakQuat` (`KismetMathLibrary.Conv_RotatorToQuaternion` (.rotation _returnvalue))))
  (bind _output_get (set `self.Information` (`KismetStringLibrary.Concat_StrStr` (`self.Topic Prefix`) "," (`KismetStringLibrary.Conv_NameToString` (`self.RobotSelection`)) "," (`KismetStringLibrary.Conv_ObjectToString` (`SkinnedMeshComponent.GetSkinnedAsset` (`self.Arm`))) "," (`KismetStringLibrary.Conv_TransformToString` (`SceneComponent.K2_GetComponentToWorld` (`self.Arm`))) "," (`KismetStringLibrary.Conv_DoubleToString` (`SceneCaptureComponent2D.FOVAngle` (`self.Color`))) "," (`KismetStringLibrary.Conv_IntToString` (`self.ImageHeight`)) "," (`KismetStringLibrary.Conv_IntToString` (`self.ImageWidth`)) "," (`KismetStringLibrary.Conv_TransformToString` _returnvalue) "," (`KismetStringLibrary.BuildString_Double` (`KismetStringLibrary.BuildString_Double` (`KismetStringLibrary.BuildString_Double` (`KismetStringLibrary.BuildString_Double` "Camera Quat: " "X=" _returnvalue_x) "Y=" _returnvalue_y) "Z=" _returnvalue_z) "W=" _returnvalue_w))))
  (return _output_get))

(fn `UserConstructionScript`)