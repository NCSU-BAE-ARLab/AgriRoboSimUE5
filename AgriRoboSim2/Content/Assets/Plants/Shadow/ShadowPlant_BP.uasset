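; Plant actor that builds a visible mesh and a segmentation twin from OBJ/MTL data through its ROS2LoadModel component.
; Tick feeds queued OBJ text and advances construction in chunks, publishing load state until finished.
; BuildMaterial then paints per-material render-target grids: colors or seeded random LeafDT leaf textures for appearance, and GameState-issued ID colors for segmentation.
; Leaf atlases are exported as PNGs; the data-table static-mesh swap path is disconnected.
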(event `self.ReceiveTick`
  (params (DeltaSeconds :type "Float (single-precision)"))
  (if (`self.Stop`)
    (`TextRenderComponent.K2_SetText` (`self.TextRender`) "1")
    (else
      (`self.RebuildModelAsync`)))
  (bind _outactors (`GameplayStatics.GetAllActorsOfClass` "/Game/Robot/Robot_BP.Robot_BP_C"))
  (for _array_element _outactors
    (bind _returnvalue (`self.K2_GetActorLocation` _array_element))
    (if (> (`KismetMathLibrary.Vector_Distance` _returnvalue (0.0 0.0 400.0)) 100.0)
      (`TextRenderComponent.K2_SetText` (`self.TextRender`) (`KismetTextLibrary.Conv_DoubleToText` (.x _returnvalue) "HalfToEven")))))

(event `self.ReceiveBeginPlay`
  (set `DynamicPlantMesh.CompletedLoad` true (`self.ROS2LoadModel`)))

(event `ChangePlant`
  (params (Row :type Integer :default 1)))

(fn `BuildMaterial`
  (locals (MaterialData :type String) (MaterialSemantic :type String) (MaterialSecIdx :type Integer) (RandomGen :type "RandomStream Structure"))
  (bind _ros2loadmodel (`self.ROS2LoadModel`))
  (bind _leafdt (`self.LeafDT`))
  (bind _randomgen (`local.RandomGen`))
  (bind _leafdt_2 (`self.LeafDT`))
  (bind _randomgen_2 (`local.RandomGen`))
  (bind (_lefts _rights _returnvalue) (`KismetStringLibrary.Split` (`local.MaterialData`) " "))
  (bind _returnvalue_2 (`KismetMathLibrary.Max` (`self.TextureGridCount`) 1))
  (bind _returnvalue_3 (`KismetMathLibrary.Max` (`self.TextureGridCount`) 1))
  (bind _returnvalue_4 (`KismetMathLibrary.Max` (`self.TextureGridCount`) 1))
  (bind (_lefts_2 _rights_2) (`KismetStringLibrary.Split` _rights " "))
  (bind _returnvalue_5 (* _returnvalue_4 _returnvalue_4))
  (bind _returnvalue_6 (* _returnvalue_3 _returnvalue_3))
  (bind _returnvalue_7 (* (`KismetMathLibrary.Max` (`self.TextureGridCount`) 1) 256))
  (bind _returnvalue_8 (* (`KismetMathLibrary.Max` (`self.TextureGridCount`) 1) 2))
  (bind _returnvalue_9 (* (`KismetMathLibrary.Max` (`self.TextureGridCount`) 1) 2))
  ;[1 1 1] For Each Material From the MTL file
  (for (_array_element _array_index) (`DynamicPlantMesh.OBJMaterialName` _ros2loadmodel)
    (set `local.MaterialSemantic` _array_element)
    (set `local.MaterialSecIdx` _array_index)
    (set `local.MaterialData` (`|GetArrayItem` (`DynamicPlantMesh.MTLMaterialDef` _ros2loadmodel) (`KismetArrayLibrary.Array_Find` (`DynamicPlantMesh.MTLMaterialName` _ros2loadmodel) _array_element)))
    (if _returnvalue
      (`|ExecutionSequence`
        (:`then_0`
          ;[1 1 1] RGB, normal appearance
          (bind _returnvalue_10 (`KismetMaterialLibrary.CreateDynamicMaterialInstance` "/Game/Assets/Plants/procedural/main/VertexColorMat.VertexColorMat" "None"))
          (bind _returnvalue_11 (`KismetRenderingLibrary.CreateRenderTarget2D` _returnvalue_8 _returnvalue_8 "RTF_RGBA8"))
          (bind (_canvas _size _context) (`KismetRenderingLibrary.BeginDrawCanvasToRenderTarget` _returnvalue_11))
          (for _index (range 1 (+ _returnvalue_6 1))
            (bind (_startx _starty) (`/Game/Assets/Helper/InstanceManager_BFL.IdxToScreenPos` _index _returnvalue_3))
            (`Canvas.K2_DrawBox` _canvas (`KismetMathLibrary.MakeVector2D` _startx _starty) (1.0 1.0) 1.0 (`KismetMathLibrary.MakeColor` (`KismetStringLibrary.Conv_StringToDouble` _lefts) (`KismetStringLibrary.Conv_StringToDouble` _lefts_2) (`KismetStringLibrary.Conv_StringToDouble` _rights_2))))
          (`KismetRenderingLibrary.EndDrawCanvasToRenderTarget` _context)
          (`KismetArrayLibrary.Array_Add` (`self.VertexColorRT`) _returnvalue_11)
          (`MaterialInstanceDynamic.SetTextureParameterValue` _returnvalue_10 "Texture" _returnvalue_11)
          (`PrimitiveComponent.SetMaterial` (`self.DynamicMesh`) (`local.MaterialSecIdx`) _returnvalue_10))
        (:`then_1`
          ;[1 1 1] Semantic, instance
          (bind _returnvalue_12 (`KismetMaterialLibrary.CreateDynamicMaterialInstance` "/Game/Assets/Plants/procedural/main/VertexColorMat.VertexColorMat"))
          (bind _returnvalue_13 (`KismetRenderingLibrary.CreateRenderTarget2D` _returnvalue_9 _returnvalue_9 "RTF_RGBA8"))
          (set `Texture.MipLoadOptions` "OnlyFirstMip" _returnvalue_13)
          (set `Texture.Filter` "TF_Nearest" _returnvalue_13)
          (set `Texture.CompressionSettings` "TC_EditorIcon" _returnvalue_13)
          (set `Texture.SRGB` false _returnvalue_13)
          (set `Texture.bUseLegacyGamma` false _returnvalue_13)
          (bind (_canvas_2 _size_2 _context_2) (`KismetRenderingLibrary.BeginDrawCanvasToRenderTarget` _returnvalue_13))
          (for _index_2 (range 1 (+ _returnvalue_6 1))
            (bind _asmain_game_state_base (cast `/Game/Levels/GameModes/MainMenu/MainGameStateBase` (`GameplayStatics.GetGameState`)))
            (bind (_idr _idg _idb) (`/Game/Levels/GameModes/MainMenu/MainGameStateBase.ObtainNextID` _asmain_game_state_base (`local.MaterialSemantic`) 1))
            (bind (_startx_2 _starty_2) (`/Game/Assets/Helper/InstanceManager_BFL.IdxToScreenPos` _index_2 _returnvalue_3))
            (`Canvas.K2_DrawBox` _canvas_2 (`KismetMathLibrary.MakeVector2D` _startx_2 _starty_2) (1.0 1.0) 1.0 (`KismetMathLibrary.MakeColor` (/ (`KismetMathLibrary.Conv_IntToDouble` _idr) 255.0) (/ (`KismetMathLibrary.Conv_IntToDouble` _idg) 255.0) (/ (`KismetMathLibrary.Conv_IntToDouble` _idb) 255.0))))
          (`KismetRenderingLibrary.EndDrawCanvasToRenderTarget` _context_2)
          (`KismetArrayLibrary.Array_Add` (`self.VertexColorRT`) _returnvalue_13)
          (`MaterialInstanceDynamic.SetTextureParameterValue` _returnvalue_12 "Texture" _returnvalue_13)
          (`PrimitiveComponent.SetMaterial` (`self.DynamicMeshSeg`) (`local.MaterialSecIdx`) _returnvalue_12)))
      (else
        (`|ExecutionSequence`
          (:`then_0`
            (bind _returnvalue_14 (`KismetMaterialLibrary.CreateDynamicMaterialInstance` "/Game/Assets/Plants/procedural/main/ProceduralMeshMat.ProceduralMeshMat"))
            (bind _returnvalue_15 (`KismetRenderingLibrary.CreateRenderTarget2D` _returnvalue_7 _returnvalue_7 "RTF_RGBA8"))
            (set `Texture.MipLoadOptions` "OnlyFirstMip" _returnvalue_15)
            (set `Texture.Filter` "TF_Nearest" _returnvalue_15)
            (bind (_canvas_3 _size_3 _context_3) (`KismetRenderingLibrary.BeginDrawCanvasToRenderTarget` _returnvalue_15))
            (bind _outrownames (`DataTableFunctionLibrary.GetDataTableRowNames` _leafdt_2))
            (`KismetMathLibrary.SetRandomStreamSeed` _randomgen_2)
            (for _index_3 (range 1 (+ _returnvalue_5 1))
              (bind _returnvalue_16 (`|GetDataTableRow` _leafdt_2 (`|GetArrayItem` _outrownames (`KismetMathLibrary.RandomIntegerInRangeFromStream` _randomgen_2 0 (- (`KismetArrayLibrary.Array_Length` _outrownames) 1))))
                (:`then`
                  (bind (_startx_3 _starty_3) (`/Game/Assets/Helper/InstanceManager_BFL.IdxToScreenPos` _index_3 _returnvalue_2 256))
                  (bind (_texture _croptype _variant _disease _cropid _diseaseid _stementry _rotationtohorizontal) (break `/Game/Assets/DataTables/GenericLeaf_S` _returnvalue_16))
                  (bind _returnvalue_17 (`KismetSystemLibrary.LoadAsset_Blocking` _texture))
                  (bind _astexture_2d (cast `Texture2D` _returnvalue_17))
                  (`Canvas.K2_DrawTexture` _canvas_3 _astexture_2d (`KismetMathLibrary.MakeVector2D` (+ _startx_3 1.0) (+ _starty_3 1.0)) (254.0 254.0) (0.0 0.0) (1.0 1.0) (struct :`R` 1.0 :`G` 1.0 :`B` 1.0) "BLEND_Masked" _rotationtohorizontal _stementry))))
            (`KismetRenderingLibrary.EndDrawCanvasToRenderTarget` _context_3)
            (`KismetArrayLibrary.Array_Add` (`self.VertexColorRT`) _returnvalue_15)
            (`MaterialInstanceDynamic.SetTextureParameterValue` _returnvalue_14 "Texture" _returnvalue_15)
            (`PrimitiveComponent.SetMaterial` (`self.DynamicMesh`) (`local.MaterialSecIdx`) _returnvalue_14)
            (`KismetRenderingLibrary.ExportRenderTarget` _returnvalue_15 (`BlueprintPathsLibrary.ProjectSavedDir`) (`KismetStringLibrary.Concat_StrStr` "leaf" "_" (`KismetStringLibrary.Conv_IntToString` (`local.MaterialSecIdx`)) ".png")))
          (:`then_1`
            (bind _returnvalue_18 (`KismetMaterialLibrary.CreateDynamicMaterialInstance` "/Game/Assets/Plants/procedural/main/ProceduralMeshMat.ProceduralMeshMat"))
            (bind _returnvalue_19 (`KismetRenderingLibrary.CreateRenderTarget2D` _returnvalue_7 _returnvalue_7 "RTF_RGBA8"))
            (set `Texture.MipLoadOptions` "OnlyFirstMip" _returnvalue_19)
            (set `Texture.Filter` "TF_Nearest" _returnvalue_19)
            (set `Texture.CompressionSettings` "TC_EditorIcon" _returnvalue_19)
            (set `Texture.SRGB` false _returnvalue_19)
            (set `Texture.bUseLegacyGamma` false _returnvalue_19)
            (`KismetSystemLibrary.PrintString` (`KismetStringLibrary.Conv_ByteToString` (`Texture.LODGroup` _returnvalue_19)))
            (bind (_canvas_4 _size_4 _context_4) (`KismetRenderingLibrary.BeginDrawCanvasToRenderTarget` _returnvalue_19))
            (bind _outrownames_2 (`DataTableFunctionLibrary.GetDataTableRowNames` _leafdt))
            (`KismetMathLibrary.SetRandomStreamSeed` _randomgen)
            (for _index_4 (range 1 (+ _returnvalue_5 1))
              (bind _returnvalue_20 (`|GetDataTableRow` _leafdt (`|GetArrayItem` _outrownames_2 (`KismetMathLibrary.RandomIntegerInRangeFromStream` _randomgen 0 (- (`KismetArrayLibrary.Array_Length` _outrownames_2) 1))))
                (:`then`
                  (bind _asmain_game_state_base_2 (cast `/Game/Levels/GameModes/MainMenu/MainGameStateBase` (`GameplayStatics.GetGameState`)))
                  (bind (_texture_2 _croptype_2 _variant_2 _disease_2) (break `/Game/Assets/DataTables/GenericLeaf_S` _returnvalue_20))
                  (bind (_idr_2 _idg_2 _idb_2) (`/Game/Levels/GameModes/MainMenu/MainGameStateBase.ObtainNextID` _asmain_game_state_base_2 (`KismetStringLibrary.Concat_StrStr` (`local.MaterialSemantic`) "_" (`KismetStringLibrary.Conv_IntToString` _index_4) "_" _croptype_2 "_" _variant_2 "_" _disease_2) 1))
                  (bind (_startx_4 _starty_4) (`/Game/Assets/Helper/InstanceManager_BFL.IdxToScreenPos` _index_4 _returnvalue_2 256))
                  (bind _returnvalue_21 (+ _startx_4 128.0))
                  (bind _returnvalue_22 (+ _starty_4 128.0))
                  (bind _linearcolor (make `LinearColor` (/ (`KismetMathLibrary.Conv_IntToDouble` _idr_2) 255.0) (/ (`KismetMathLibrary.Conv_IntToDouble` _idg_2) 255.0) (/ (`KismetMathLibrary.Conv_IntToDouble` _idb_2) 255.0) 1.0))
                  (`Canvas.K2_DrawLine` _canvas_4 (`KismetMathLibrary.MakeVector2D` _returnvalue_21 _returnvalue_22) (`KismetMathLibrary.MakeVector2D` (+ _returnvalue_21 255.0) _returnvalue_22) 256.0 _linearcolor)
                  (`KismetSystemLibrary.PrintString` (`KismetStringLibrary.Conv_ColorToString` _linearcolor)))))
            (`KismetRenderingLibrary.EndDrawCanvasToRenderTarget` _context_4)
            (`KismetArrayLibrary.Array_Add` (`self.VertexColorRT`) _returnvalue_19)
            (`MaterialInstanceDynamic.SetTextureParameterValue` _returnvalue_18 "Texture" _returnvalue_15)
            (`MaterialInstanceDynamic.SetTextureParameterValue` _returnvalue_18 "TextureInstance" _returnvalue_19)
            (`MaterialInstanceDynamic.SetScalarParameterValue` _returnvalue_18 "bSegmentation" 1.0)
            (`PrimitiveComponent.SetMaterial` (`self.DynamicMeshSeg`) (`local.MaterialSecIdx`) _returnvalue_18)
            (`KismetRenderingLibrary.ExportRenderTarget` _returnvalue_19 (`BlueprintPathsLibrary.ProjectSavedDir`) (`KismetStringLibrary.Concat_StrStr` "leafsegment" "_" (`KismetStringLibrary.Conv_IntToString` (`local.MaterialSecIdx`)) ".png")))))))
  (return))

(fn `GetPlantInfo`
  (set `self.Information` (`KismetStringLibrary.Concat_StrStr` (`KismetStringLibrary.Conv_TransformToString` (`SceneComponent.K2_GetComponentToWorld` (`self.DefaultSceneRoot`))) "," (`KismetSystemLibrary.GetDisplayName` (`self.StaticMesh`)) "," "" "," "" "," "" "," "" "," "" ",")))

(fn `RebuildModel`
  (bind _ros2loadmodel (`self.ROS2LoadModel`))
  (set `DynamicPlantMesh.DynMesh` (`self.DynamicMesh`) _ros2loadmodel)
  (set `DynamicPlantMesh.DynMeshSeg` (`self.DynamicMeshSeg`) _ros2loadmodel)
  (`DynamicPlantMesh.CreateMeshFromOBJString` _ros2loadmodel (`self.OBJData`) (`self.MTLData`) (`self.Flip Normal`))
  (`self.BuildMaterial`))

(fn `RebuildModelAsync`
  (bind _ros2loadmodel (`self.ROS2LoadModel`))
  (bind _ros2loadmodel_2 (`self.ROS2LoadModel`))
  (bind _ros2loadmodel_3 (`self.ROS2LoadModel`))
  (bind _ros2loadmodel_4 (`self.ROS2LoadModel`))
  (if (`DynamicPlantMesh.CompletedLoad` (`self.ROS2LoadModel`))
    (set `DynamicPlantMesh.DynMesh` (`self.DynamicMesh`) _ros2loadmodel)
    (set `DynamicPlantMesh.DynMeshSeg` (`self.DynamicMeshSeg`) _ros2loadmodel)
    (set `self.OBJData` "")
    (for _array_element (`self.OBJData_Queue`)
      (set `self.OBJData` (`KismetStringLibrary.Concat_StrStr` (`self.OBJData`) _array_element)))
    (`KismetArrayLibrary.Array_Clear` (`self.OBJData_Queue`))
    (`DynamicPlantMesh.ConfigureMeshObj` _ros2loadmodel_4 (`self.OBJData`) (`self.MTLData`))
    (else
      (bind _returnvalue (`DynamicPlantMesh.AsyncConstructMesh` _ros2loadmodel_4 250))
      (bind _returnvalue_2 (`DynamicPlantMesh.CurrentProgress` (`self.ROS2LoadModel`)))
      (`TextRenderComponent.K2_SetText` (`self.TextRender`) (`KismetTextLibrary.Conv_DoubleToText` _returnvalue_2 "HalfToEven"))
      (if _returnvalue
        (`DynamicPlantMesh.FinalizeMesh` (`self.ROS2LoadModel`))
        (set `self.Stop` true)
        (`self.BuildMaterial`)
        (`ROS2LoadModel.PublishState` _ros2loadmodel_2 (`KismetStringLibrary.Concat_StrStr` "Loaded:" (`KismetStringLibrary.Conv_BoolToString` (`DynamicPlantMesh.CompletedLoad` _ros2loadmodel_2))))
        (set `self.Ready` true)
        (else
          (`ROS2LoadModel.PublishState` _ros2loadmodel_3 (`KismetStringLibrary.Concat_StrStr` "Loaded:" (`KismetStringLibrary.Conv_IntToString` (`DynamicPlantMesh.AsyncLoadLine` _ros2loadmodel_3)))))))))

(fn `UserConstructionScript`
  (bind _dynamicmesh (`self.DynamicMesh`))
  (bind _ros2loadmodel (`self.ROS2LoadModel`))
  (set `DynamicPlantMesh.DynMesh` _dynamicmesh _ros2loadmodel)
  (set `DynamicPlantMesh.DynMeshSeg` (`self.DynamicMeshSeg`) _ros2loadmodel)
  (set `BaseDynamicMeshComponent.bEnableFlatShading` (`self.Flat Shading`) _dynamicmesh))