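; Procedural plant actor that builds its mesh from OBJ and MTL string data in the construction script.
; A ProceduralPlantMesh helper fills the ProceduralMesh component and returns the material names and definitions.
; Each OBJ material gets a dynamic instance, either a vertex color material tinted with RGB split from its definition, or a leaf material textured from a MaterialMap data table lookup.
; Missing table rows fall back to the plain procedural mesh material.
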(fn `UserConstructionScript`
  (set `ProceduralPlantMesh.ProcMesh` (`self.ProceduralMesh`) (`self.ProceduralPlantMesh`))
  (bind (_mtlmaterialname _mtlmaterialdef _objmaterialname) (`ProceduralPlantMesh.CreateMeshFromOBJString` (`self.ProceduralPlantMesh`) (`self.ObjData`) (`self.MTLData`) (`self.Flip Normal`)))
  (for (_array_element _array_index) _objmaterialname
    (bind _output (`|GetArrayItem` _mtlmaterialdef (`KismetArrayLibrary.Array_Find` _mtlmaterialname _array_element)))
    (`KismetSystemLibrary.PrintString` _output)
    (bind (_lefts _rights _returnvalue) (`KismetStringLibrary.Split` _output " "))
    (if _returnvalue
      (bind _returnvalue_2 (`KismetMaterialLibrary.CreateDynamicMaterialInstance` "/Game/Assets/Plants/procedural/main/VertexColorMat.VertexColorMat" "None"))
      (bind (_lefts_2 _rights_2) (`KismetStringLibrary.Split` _rights " "))
      (`MaterialInstanceDynamic.SetVectorParameterValue` _returnvalue_2 "Color" (make `LinearColor` (`KismetStringLibrary.Conv_StringToDouble` _lefts) (`KismetStringLibrary.Conv_StringToDouble` _lefts_2) (`KismetStringLibrary.Conv_StringToDouble` _rights_2) 1.0))
      (bind _returnvalue_3 (+ _array_index 1))
      (`PrimitiveComponent.SetMaterial` (`self.ProceduralMesh`) _returnvalue_3 _returnvalue_2)
      (else
        (bind _returnvalue_4 (`KismetMaterialLibrary.CreateDynamicMaterialInstance` "/Game/Assets/Plants/procedural/main/ProceduralMeshMat.ProceduralMeshMat"))
        (bind _returnvalue_5 (`|GetDataTableRow` (`self.MaterialMap`) (`KismetStringLibrary.Conv_StringToName` _output))
          (:`then`
            (`MaterialInstanceDynamic.SetTextureParameterValue` _returnvalue_4 "Leaf" (`.Texture_5_F92719494D41D31D471760B8D8C78B85` (break `/Game/Assets/Plants/procedural/main/BaseLeafAssets` _returnvalue_5)))
            (`PrimitiveComponent.SetMaterial` (`self.ProceduralMesh`) _returnvalue_3 _returnvalue_4))
          (:`RowNotFound`
            (`PrimitiveComponent.SetMaterial` (`self.ProceduralMesh`) _returnvalue_3 "/Game/Assets/Plants/procedural/main/ProceduralMeshMat.ProceduralMeshMat")))))))