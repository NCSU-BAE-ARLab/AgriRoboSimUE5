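; Plant actor that swaps its mesh for generating colored or segmentation plant images.
; ChangePlant looks up the selection in a plant data table, applies mesh and scale, and returns the plant name.
; For segment-tagged actors it shows the plant only in scene captures and applies a dynamic material with the segmentation texture, optionally whitening the ORT map.
; The material loop returns on its first pass, so only the first slot changes.
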(event `self.ReceiveBeginPlay`)

(fn `ChangePlant`
  (params (PlantSelection :type Integer) (ClearOpactiy :type Boolean))
  (returns (PlantName :type String))
  (locals (NewLocalVar :type "StaticMaterial Structure"))
  (bind _plantmesh (`self.PlantMesh`))
  (`KismetSystemLibrary.PrintString` "Change Plant")
  (bind _returnvalue (`|GetDataTableRow` "/Game/Assets/Plants/2-plant-vis/PlantCollection_DT.PlantCollection_DT" (`KismetStringLibrary.Conv_StringToName` (`KismetStringLibrary.Conv_IntToString` PlantSelection)))
    (:`then`
      (bind _output (`|ConvertAsset` (`.Mesh_21_C61ED59E4333D2C6C8B34985FFF4948E` (break `/Game/Assets/Plants/2-plant-vis/PlantAuto_S` _returnvalue))))
      (`StaticMeshComponent.SetStaticMesh` (`self.MeshHold`) _output)
      (`StaticMeshComponent.SetStaticMesh` _plantmesh _output)
      (`SceneComponent.SetWorldScale3D` _plantmesh (`KismetMathLibrary.Conv_DoubleToVector` (break `/Game/Assets/Plants/2-plant-vis/PlantAuto_S` _returnvalue)))
      (`|ExecutionSequence`
        (:`then_0`
          (if (`self.ActorHasTag` "ColoredImageGen")
            (bind _returnvalue_2 (`KismetTextLibrary.Conv_TextToString` (`.Name_7_5C4A3A3245FEDBE223E9DFBD058681B7` (break `/Game/Assets/Plants/2-plant-vis/PlantAuto_S` _returnvalue))))
            (return _returnvalue_2)))
        (:`then_1`
          (if (`self.ActorHasTag` "SegmentImageGen")
            (`PrimitiveComponent.SetVisibleInSceneCaptureOnly` (`self.PlantMesh`) true)
            (for (_array_element _array_index) (`MeshComponent.GetMaterials` (`self.MeshHold`))
              (bind _returnvalue_3 (`KismetMaterialLibrary.CreateDynamicMaterialInstance` _array_element "Temp"))
              (`MaterialInstanceDynamic.SetScalarParameterValue` _returnvalue_3 "OpacityIntensity" 0.2)
              (`MaterialInstanceDynamic.SetTextureParameterValue` _returnvalue_3 "Albedo" (`.SegmentationTexture_23_5E3E46A24DC79C441479689CC3CF61BD` (break `/Game/Assets/Plants/2-plant-vis/PlantAuto_S` _returnvalue)))
              (if (`local.ClearOpactiy`)
                (`MaterialInstanceDynamic.SetTextureParameterValue` _returnvalue_3 "ORT" "/Game/MSPresets/M_MS_Glass_Material/Textures/White.White"))
              (`PrimitiveComponent.SetMaterial` (`self.PlantMesh`) _array_index _returnvalue_3)
              (return _returnvalue_2))))))
    (:`RowNotFound`
      (return "PlantNotFound"))))

(fn `UserConstructionScript`)