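; UR10e robot arm Blueprint that moves a camera, captures color and segmentation images, and marks seen plant surfaces.
; Tick drives six physics-constraint motors from ROS vectors or timed default inputs and records end-effector position for ROS.
; A camera line trace passes hit UVs to BP_Plant or BP_Cylinder.
; TakeData captures tag-filtered scenes into fresh render targets; clearing it exports JPEGs and a camera-pose CSV per arm ID.
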(event `self.ReceiveBeginPlay`
  (bind _motorstrength (`self.MotorStrength`))
  (bind _datacapturescene2d (`self.DataCaptureScene2D`))
  (bind _segmcapturescene2d (`self.SegmCaptureScene2d`))
  (set `self.MotorRatio` 75.0)
  (set `self.MotorStrength` 2000.0)
  (`PhysicsConstraintComponent.SetAngularDriveParams` (`self.joint4`) (* (`self.MotorRatio`) _motorstrength 0.5) _motorstrength 100000.0)
  (`PhysicsConstraintComponent.SetAngularDriveParams` (`self.joint5`) (* (`self.MotorRatio`) _motorstrength 0.5) _motorstrength 100000.0)
  (`PhysicsConstraintComponent.SetAngularDriveParams` (`self.joint6`) (* (`self.MotorRatio`) _motorstrength 0.5) _motorstrength 100000.0)
  (`PhysicsConstraintComponent.SetAngularDriveParams` (`self.joint1`) (* (`self.MotorRatio`) _motorstrength 1.0) _motorstrength 1000.0)
  (`PhysicsConstraintComponent.SetAngularDriveParams` (`self.joint2`) (* (`self.MotorRatio`) _motorstrength 1.0) _motorstrength 1000.0)
  (`PhysicsConstraintComponent.SetAngularDriveParams` (`self.joint3`) (* (`self.MotorRatio`) _motorstrength 0.85) _motorstrength 0.0)
  (set `self.ArmID` (`self.ArmID_BP`))
  (bind _desiredview (`CameraComponent.GetCameraView` (`self.RobotCam`) 0.0))
  (bind (_location _rotation _fov _orthowidth _orthonearclipplane _orthofarclipplane _perspectivenearclipplane _aspectratio _bconstrainaspectratio _busefieldofviewforlod _projectionmode _postprocessblendweight _postprocesssettings) (break `MinimalViewInfo` _desiredview))
  (bind _output_get (set `SceneCaptureComponent2D.ProjectionType` _projectionmode _datacapturescene2d))
  (bind _output_get_2 (set `SceneCaptureComponent2D.FOVAngle` _fov _datacapturescene2d))
  (bind _output_get_3 (set `SceneCaptureComponent2D.PostProcessSettings` _postprocesssettings _datacapturescene2d))
  (bind _output_get_4 (set `SceneCaptureComponent2D.PostProcessBlendWeight` _postprocessblendweight _datacapturescene2d))
  (set `SceneCaptureComponent2D.ProjectionType` _output_get _segmcapturescene2d)
  (set `SceneCaptureComponent2D.FOVAngle` _output_get_2 _segmcapturescene2d)
  (set `SceneCaptureComponent2D.PostProcessSettings` _output_get_3 _segmcapturescene2d)
  (set `SceneCaptureComponent2D.PostProcessBlendWeight` _output_get_4 _segmcapturescene2d)
  (bind _outactors (`GameplayStatics.GetAllActorsWithTag` "SegmentImageGen"))
  (set `SceneCaptureComponent.ShowOnlyActors` _outactors (`self.SegmCaptureScene2d`))
  (bind _outactors_2 (`GameplayStatics.GetAllActorsWithTag` "ColoredImageGen"))
  (set `SceneCaptureComponent.ShowOnlyActors` _outactors_2 (`self.DataCaptureScene2D`)))

(event `self.ReceiveTick`
  (params (DeltaSeconds :type "Float (single-precision)"))
  (bind _readytosave (`self.ReadyToSave`))
  (bind _datacapturescene2d (`self.DataCaptureScene2D`))
  (bind _segmcapturescene2d (`self.SegmCaptureScene2d`))
  ;[1 1 1] MainLoop
  (`self.CountTime_Event` DeltaSeconds (`self.CycleTimeConst`))
  (if (`self.UseROS`)
    (`self.UseROSInputs_Event` (`self.ArmID`))
    (else
      (`self.DefaultInputs_Event` (`self.CountTimeTrigger`))))
  (`self.UpdateArmPosition_Event`)
  (`self.DrawSeenPlant`)
  (`self.CheckArmPosition_Event`)
  (if (`self.takeData`)
    (if _readytosave
      (`SceneCaptureComponent2D.CaptureScene` _datacapturescene2d)
      (`SceneCaptureComponent2D.CaptureScene` _segmcapturescene2d)
      (else
        (set `self.ReadyToSave` true)
        (`self.Refresh RT` _datacapturescene2d)
        (`self.Refresh RT` _segmcapturescene2d)))
    (elif _readytosave
      (set `self.ReadyToSave` false)
      (`self.TakeData_Event` _datacapturescene2d "Color")
      (`self.TakeData_Event` _segmcapturescene2d "Segment")
      (`KismetSystemLibrary.PrintString` "Done"))))

(event `UseROSInputs_Event`
  (params (ID :type Integer))
  ;[1 1 1] ROS Vec3 Inputs to set joint angles
  (set `self.Joint1Rotator` (`KismetMathLibrary.MakeRotator` 0.0 (.x (`self.firstSet`))))
  (set `self.Joint2Roator` (`KismetMathLibrary.MakeRotator` 0.0 0.0 (.y (`self.firstSet`))))
  (set `self.Joint3Rotator` (`KismetMathLibrary.MakeRotator` 0.0 0.0 (.z (`self.firstSet`))))
  (set `self.Joint4Rotator` (`KismetMathLibrary.MakeRotator` 0.0 0.0 (.x (`self.secondSet`))))
  (set `self.Joint5Rotator` (`KismetMathLibrary.MakeRotator` 0.0 (.y (`self.secondSet`))))
  (set `self.Joint6Rotator` (`KismetMathLibrary.MakeRotator` 0.0 0.0 (.z (`self.secondSet`)))))

(event `CheckArmPosition_Event`
  ;[1 1 1] Get World Position of the last joint (for publish in ROS)
  (set `self.eefJointPos` (`SceneComponent.K2_GetComponentLocation` (`self.EEF`))))

(event `TakeData_Event`
  (params (SceneCap2d :type "SceneCaptureComponent2D Object Reference") (ImgType :type String))
  (bind _datacapturescene2d (`self.DataCaptureScene2D`))
  (bind _camlocationarr (`self.CamLocationArr`))
  (bind _returnvalue (`KismetStringLibrary.Conv_IntToString` (`self.ArmID`)))
  (bind _returnvalue_2 (`KismetStringLibrary.Concat_StrStr` (`KismetSystemLibrary.GetProjectSavedDirectory`) "Test"))
  (bind _returnvalue_3 (+ (`self.ImageCount`) 1))
  (bind (_x _y _z) (`KismetMathLibrary.BreakVector3f` (`SceneComponent.K2_GetComponentLocation` _datacapturescene2d)))
  (bind (_x_2 _y_2 _z_2 _w) (`KismetMathLibrary.BreakQuat` (`KismetMathLibrary.Conv_RotatorToQuaternion` (`SceneComponent.K2_GetComponentRotation` _datacapturescene2d))))
  ;[1 1 1] Generate Image and Text Data
  (`KismetRenderingLibrary.ExportRenderTarget` (`SceneCaptureComponent2D.TextureTarget` SceneCap2d) _returnvalue_2 (`KismetStringLibrary.Concat_StrStr` _returnvalue "_" (`KismetStringLibrary.Conv_IntToString` _returnvalue_3) "_" ImgType ".jpeg"))
  (set `self.ImageCount` _returnvalue_3)
  (`KismetArrayLibrary.Array_Append` _camlocationarr (`|MakeArray` (`KismetStringLibrary.BuildString_Int` (`KismetStringLibrary.BuildString_Int` (`KismetStringLibrary.BuildString_Double` (`KismetStringLibrary.BuildString_Double` (`KismetStringLibrary.BuildString_Double` (`KismetStringLibrary.BuildString_Double` (`KismetStringLibrary.BuildString_Double` (`KismetStringLibrary.BuildString_Double` (`KismetStringLibrary.BuildString_Double` ImgType "," _x ",") "" _y ",") "" _z ",") "" _x_2 ",") "" _y_2 ",") "" _z_2 ",") "" _w ",") "" (`self.ArmID`) ",") "" (`self.ImageCount`) ",")))
  (`self.saveCamData` (`KismetStringLibrary.Concat_StrStr` _returnvalue_2 "//" _returnvalue "camLocation.csv") _camlocationarr))

(event `DefaultInputs_Event`
  (params (RandomVal :type "Boolean (by ref)"))
  (bind _randomval (`self.RandomVal`))
  ;[1 1 1] Default Inputs to set joint angles
  (if RandomVal
    (set `self.RandomVal` 180.0))
  (set `self.Joint1Rotator` (`KismetMathLibrary.MakeRotator` 0.0 _randomval))
  (set `self.Joint2Roator` (`KismetMathLibrary.MakeRotator` 0.0 0.0 _randomval))
  (set `self.Joint3Rotator` (`KismetMathLibrary.MakeRotator` 0.0 0.0 _randomval))
  (set `self.Joint4Rotator` (`KismetMathLibrary.MakeRotator` 0.0 0.0 _randomval))
  (set `self.Joint5Rotator` (`KismetMathLibrary.MakeRotator` 0.0 _randomval))
  (set `self.Joint6Rotator` (`KismetMathLibrary.MakeRotator` 0.0 0.0 _randomval))
  (`KismetSystemLibrary.PrintString` (`KismetStringLibrary.Conv_DoubleToString` _randomval)))

(event `UpdateArmPosition_Event`
  ;[1 1 1] UpdateArmPosition
  (`PhysicsConstraintComponent.SetAngularOrientationTarget` (`self.joint1`) (`self.Joint1Rotator`))
  (`PhysicsConstraintComponent.SetAngularOrientationTarget` (`self.joint2`) (`self.Joint2Roator`))
  (`PhysicsConstraintComponent.SetAngularOrientationTarget` (`self.joint3`) (`self.Joint3Rotator`))
  (`PhysicsConstraintComponent.SetAngularOrientationTarget` (`self.joint4`) (`self.Joint4Rotator`))
  (`PhysicsConstraintComponent.SetAngularOrientationTarget` (`self.joint5`) (`self.Joint5Rotator`))
  (`PhysicsConstraintComponent.SetAngularOrientationTarget` (`self.joint6`) (`self.Joint6Rotator`)))

(event `CountTime_Event`
  (params (DeltaSeconds :type "Float (double-precision) (by ref)") (CountSeconds :type "Float (double-precision) (by ref)"))
  (bind _cycletime (`self.CycleTime`))
  (bind _returnvalue (+ DeltaSeconds _cycletime))
  (bind _returnvalue_2 (> _returnvalue CountSeconds))
  ;[1 1 1] Time Trigger Once
  (set `self.CycleTime` _returnvalue)
  (set `self.CountTimeTrigger` _returnvalue_2)
  (if _returnvalue_2
    (set `self.CycleTime` (- _cycletime CountSeconds -1.0))))

(fn `DrawSeenPlant`
  (bind _robotcam (`self.RobotCam`))
  (bind _returnvalue (`SceneComponent.K2_GetComponentLocation` _robotcam))
  (bind (_outhit _returnvalue_2) (`KismetSystemLibrary.LineTraceSingle` _returnvalue (+ _returnvalue (* (`SceneComponent.GetForwardVector` _robotcam) 200.0)) "TraceTypeQuery2"))
  (if _returnvalue_2
    (bind (_bblockinghit _binitialoverlap _time _distance _location _impactpoint _normal _impactnormal _physmat _hitactor) (`GameplayStatics.BreakHitResult` _outhit))
    (bind _asbp_plant (cast `/Game/Assets/Painting/BP_Plant` _hitactor)
      (:`then`
        (bind _uv (`GameplayStatics.FindCollisionUV` _outhit))
        (`/Game/Assets/Painting/BP_Plant.SeenArea` _asbp_plant _uv))
      (:`CastFailed`
        (bind _asbp_cylinder (cast `/Game/Assets/Painting/BP_Cylinder` _hitactor))
        (`/Game/Assets/Painting/BP_Cylinder.SeenArea` _asbp_cylinder _uv)))))

(fn `Refresh RT`
  (params (SceneCap2D :type "SceneCaptureComponent2D Object Reference"))
  (bind _returnvalue (`KismetRenderingLibrary.CreateRenderTarget2D` 1920 1080 "RTF_RGBA8"))
  (set `TextureRenderTarget.TargetGamma` 2.5 _returnvalue)
  (bind _output_get (set `self.camImage` _returnvalue))
  (set `SceneCaptureComponent2D.TextureTarget` _output_get SceneCap2D)
  (`KismetSystemLibrary.PrintString` "TakingPic" true true (struct :`G` 0.66 :`B` 1.0 :`A` 1.0) 0.5))

(fn `UserConstructionScript`)